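; Ranger enemy projectile that launches at TargetActor and, on box overlap, sends a damage message, spawns an explosion and destroys itself.
; BeginPlay sets lifespan, solves a straight shot to above the target, then activates ProjectileMovement using normalized actor location plus that offset as velocity.
; Tick adds GravityScale to the Visual's vertical physics velocity.
; Quadratic, ballistic-arc and launch-velocity solvers are unused here; debug drawing remains.
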(event `self.ReceiveBeginPlay`
  (bind _returnvalue (`self.K2_GetActorLocation`))
  (bind _targetactor (`self.TargetActor`))
  (bind _projectilemovement (`self.ProjectileMovement`))
  (`self.SetLifeSpan` (`self.Lifespan`))
  (`/Engine/EditorBlueprintResources/StandardMacros.IsValid` _targetactor
    (:`Is Valid`
      (bind _result (`self.SolveStraightShotVelocity` _returnvalue (+ (`self.K2_GetActorLocation` _targetactor) (0.0 0.0 150.0))))
      (bind _returnvalue_2 (+ _returnvalue _result))
      (`KismetSystemLibrary.DrawDebugLine` _returnvalue _returnvalue_2 (struct :`R` 1.0 :`B` 0.029831 :`A` 1.0) 30.0 1.0)
      (`KismetSystemLibrary.PrintString` (`KismetStringLibrary.Conv_VectorToString` _result))
      (set `MovementComponent.Velocity` (`KismetMathLibrary.Normal` _returnvalue_2) _projectilemovement)
      (`ActorComponent.Activate` _projectilemovement true))))

(event `self.Box.OnComponentBeginOverlap`
  (params (OverlappedComponent :type "PrimitiveComponent Object Reference") (OtherActor :type "Actor Object Reference") (OtherComp :type "PrimitiveComponent Object Reference") (OtherBodyIndex :type Integer) (bFromSweep :type Boolean) (SweepResult :type "HitResult Structure (by ref)"))
  (message `/Game/Blueprints/Interfaces/Combat_Interface.DamageEvent` OtherActor)
  (`|SpawnActorFromClass` "/Game/MobileStarterContent/Blueprints/Blueprint_Effect_Explosion.Blueprint_Effect_Explosion_C" (`KismetMathLibrary.MakeTransform` SweepResult_Location) "Undefined" "OverrideRootScale" null null)
  (`self.K2_DestroyActor`))

(event `self.ReceiveTick`
  (params (DeltaSeconds :type "Float (single-precision)"))
  (`PrimitiveComponent.SetPhysicsLinearVelocity` (`self.Visual`) (`KismetMathLibrary.MakeVector` 0.0 0.0 (`self.GravityScale`)) true "None"))

(fn `SolveBallisticArcLateral`
  (params (StartPos :type "Vector Structure") (Speed :type "Float (double-precision)") (TargetPos :type "Vector Structure") (MaxHeight :type "Float (double-precision)"))
  (returns (Result :type "Vector Structure"))
  (locals (Diff :type "Vector Structure") (DiffXY :type "Vector Structure") (LateralDist :type "Float (double-precision)") (Time :type "Float (double-precision)") (FireVelocity :type "Vector Structure") (a :type "Float (double-precision)") (b :type "Float (double-precision)") (c :type "Float (double-precision)") (gravity :type "Float (double-precision)"))
  (bind _time (`local.Time`))
  (bind (_firevelocity_x _firevelocity_y) (`KismetMathLibrary.BreakVector` (`local.FireVelocity`)))
  (bind _startpos (`local.StartPos`))
  (bind (_startpos_x _startpos_y _startpos_z) (`KismetMathLibrary.BreakVector` (`local.StartPos`)))
  (bind (_targetpos_x _targetpos_y _targetpos_z) (`KismetMathLibrary.BreakVector` (`local.TargetPos`)))
  (bind _returnvalue (`KismetMathLibrary.MakeVector` _firevelocity_x _firevelocity_y (/ (+ (- (* (* -1.0 3.0) (* -1.0 (`local.a`))) (* (* -1.0 4.0) (* -1.0 (`local.b`)))) (* -1.0 (`local.c`))) (`local.Time`))))
  (`KismetSystemLibrary.DrawDebugSphere` StartPos 10.0 30 (struct :`R` 1.0 :`G` 0.775649 :`A` 1.0) 30.0 1.0)
  (`KismetSystemLibrary.DrawDebugSphere` TargetPos 10.0 30 (struct :`G` 1.0 :`B` 0.017984 :`A` 1.0) 30.0 1.0)
  (bind _output_get (set `local.Diff` (- TargetPos StartPos)))
  (bind _output_get_2 (set `local.DiffXY` (`KismetMathLibrary.MakeVector` (.x _output_get) (.y _output_get))))
  (bind _output_get_3 (set `local.LateralDist` (`KismetMathLibrary.VSize` _output_get_2)))
  (set `local.Time` (/ _output_get_3 (`local.Speed`)))
  (set `local.FireVelocity` (* (`KismetMathLibrary.Normal` (`local.DiffXY`)) (`local.Speed`)))
  (set `local.a` _startpos_z)
  (set `local.b` (`local.MaxHeight`))
  (set `local.c` _targetpos_z)
  (set `local.gravity` (/ (- (* -4.0 (`local.a`)) (+ (* -4.0 (* 2.0 (`local.b`))) (* -4.0 (`local.c`)))) (* _time _time)))
  (`KismetSystemLibrary.DrawDebugLine` _startpos (+ _startpos _returnvalue) (struct :`R` 1.0 :`B` 0.059606 :`A` 1.0) 40.0 1.0)
  (return _returnvalue))

(fn `SolveProjectileLaunchVelocity`
  (params (StartPos :type "Vector Structure") (TargetPos :type "Vector Structure") (Speed :type "Float (double-precision)"))
  (returns (Result :type "Vector Structure"))
  (locals (Proj_XY :type "Vector Structure") (Target_XY :type "Vector Structure") (Time :type "Float (double-precision)") (LateralDistance :type "Float (double-precision)") (VerticalDistance :type "Float (double-precision)") (Vz :type "Float (double-precision)") (Theta :type "Float (double-precision)") (H :type "Float (double-precision)" :default 50.0) (Vxy :type "Float (double-precision)"))
  (bind (_returnvalue_x _returnvalue_y) (`KismetMathLibrary.BreakVector` (- (`local.Target_XY`) (`local.Proj_XY`))))
  (`KismetSystemLibrary.DrawDebugSphere` StartPos 10.0 30 (struct :`R` 1.0 :`G` 0.775649 :`A` 1.0) 30.0 1.0)
  (`KismetSystemLibrary.DrawDebugSphere` TargetPos 10.0 30 (struct :`G` 1.0 :`B` 0.017984 :`A` 1.0) 30.0 1.0)
  (bind _output_get (set `local.Proj_XY` (`KismetMathLibrary.MakeVector` (.x StartPos) (.y StartPos))))
  (bind _output_get_2 (set `local.Target_XY` (`KismetMathLibrary.MakeVector` (.x TargetPos) (.y TargetPos))))
  (bind (_returnvalue_x_2 _returnvalue_y_2 _returnvalue_z) (`KismetMathLibrary.BreakVector` (- _output_get_2 _output_get)))
  (set `local.LateralDistance` (`KismetMathLibrary.VSize` (`KismetMathLibrary.MakeVector` _returnvalue_x_2 _returnvalue_y_2 _returnvalue_z)))
  (set `local.VerticalDistance` (- (.z TargetPos) (.z StartPos)))
  (set `local.Time` (+ (`KismetMathLibrary.Sqrt` (/ (* -2.0 (`local.H`)) (`self.GravityScale`))) (`KismetMathLibrary.Sqrt` (/ (* 2.0 (- (`local.VerticalDistance`) (`local.H`))) (`self.GravityScale`)))))
  (return (* (+ (* (`KismetMathLibrary.Vector_Up`) (`KismetMathLibrary.Sqrt` (* 2.0 (`local.VerticalDistance`) (`local.H`)))) (* (`KismetMathLibrary.MakeVector` _returnvalue_x _returnvalue_y) (`local.Time`))) (* (`self.GravityScale`) -1.0))))

(fn `SolveQuadratic`
  (params (c0 :type "Float (double-precision)") (c1 :type "Float (double-precision)") (c2 :type "Float (double-precision)") (s0 :type "Float (double-precision) (by ref)") (s1 :type "Float (double-precision) (by ref)"))
  (returns (val :type Integer))
  (locals (p :type "Float (double-precision)") (q :type "Float (double-precision)") (d :type "Float (double-precision)"))
  (bind _p (`local.p`))
  (set `local.p` (/ c1 (* 2.0 c0)))
  (set `local.q` (/ c2 c0))
  (bind _output_get (set `local.d` (- (* _p _p) (`local.q`))))
  (if (`KismetMathLibrary.NearlyEqual_FloatFloat` _output_get 0.0 0.001)
    (`|VariableSetRef` s1 (* (`local.p`) -1.0))
    (return 1)
    (elif (< (`local.d`) 0.0)
      (return 0)
      (else
        (`|VariableSetRef` (`local.s0`) (- (`KismetMathLibrary.Sqrt` (`local.d`)) (`local.p`)))
        (`|VariableSetRef` (`local.s1`) (- (* (`KismetMathLibrary.Sqrt` (`local.d`)) -1.0) (`local.p`)))
        (return 2)))))

(fn `SolveStraightShotVelocity`
  (params (StartPos :type "Vector Structure") (TargetPos :type "Vector Structure") (Speed :type "Float (double-precision)"))
  (returns (Result :type "Vector Structure"))
  (`KismetSystemLibrary.DrawDebugSphere` StartPos 10.0 30 (struct :`R` 1.0 :`G` 0.775649 :`A` 1.0) 30.0 1.0)
  (`KismetSystemLibrary.DrawDebugSphere` TargetPos 10.0 30 (struct :`G` 1.0 :`B` 0.017984 :`A` 1.0) 30.0 1.0)
  (return (- TargetPos StartPos)))

(fn `UserConstructionScript`)